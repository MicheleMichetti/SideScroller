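; BP_PickUpItem is a pickup item actor with a configurable mesh and a text label showing the item's name.
; The construction script applies the mesh and writes the name from its Values data into the TextRender.
; The mesh's overlap event is empty.
; Unconnected graph logic would add Values to the SideScrollerCharacter's inventory, append a W_PickUpItemSlot widget to its inventory box and destroy the actor, but never runs.
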(event OnComponentBeginOverlap(StaticMesh)
  (params (OverlappedComponent :type Primitive%20Component%20Object%20Reference) (OtherActor :type Actor%20Object%20Reference) (OtherComp :type Primitive%20Component%20Object%20Reference) (OtherBodyIndex :type Integer) (bFromSweep :type Boolean) (SweepResult :type Hit%20Result%20Structure%20%28by%20ref%29)))

(fn ConstructionScript
  (Components|StaticMesh|SetStaticMesh (Variables|Default|GetStaticMesh) (Variables|Default|GetStatic%20Mesh))
  (Rendering|Components|TextRender|SetText (Variables|Default|GetTextRender) (Utilities|Text|ToText(String) (.name (Variables|Default|GetValues)))))